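; BP_Dodge_Ball is a dodgeball actor that launches itself away from the player when it begins play, as if thrown.
; The offset from the player pawn to the ball, scaled with a stronger vertical factor, becomes a velocity-change impulse on the Dodgeball component.
; After a short delay it enables overlap events on Sphere1 to allow pickup, though that overlap handler is empty.
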(event OnComponentBeginOverlap(Sphere1)
  (params (OverlappedComponent :type Primitive%20Component%20Object%20Reference) (OtherActor :type Actor%20Object%20Reference) (OtherComp :type Primitive%20Component%20Object%20Reference) (OtherBodyIndex :type Integer) (bFromSweep :type Boolean) (SweepResult :type Hit%20Result%20Structure%20%28by%20ref%29)))

(event EventBeginPlay
  (bind _returnvalue (Game|Player|GetPlayerPawn 0))
  (bind _dodgeball (Variables|Default|GetDodgeball))
  (bind _returnvalue_2 (Transformation|GetActorLocation _returnvalue))
  (bind _returnvalue_3 (Transformation|GetWorldLocation _dodgeball))
  (bind _returnvalue_4 (- _returnvalue_3 _returnvalue_2))
  (bind (_x _y _z) (Math|Vector|BreakVector _returnvalue_4))
  (bind _returnvalue_5 (* _z 3e+01))
  (bind _returnvalue_6 (* _x 25.0))
  (bind _returnvalue_7 (* _y 25.0))
  (bind _returnvalue_8 (Math|Vector|MakeVector _returnvalue_6 _returnvalue_7 _returnvalue_5))
  (Development|PrintString (Utilities|String|ToString(Vector) _returnvalue_8))
  (Physics|AddImpulse (Variables|Default|GetDodgeball) _returnvalue_8 "None" true)
  (Utilities|FlowControl|Delay 1.0)
  (Development|PrintString "I can be picked up now")
  (Variables|/Script/Engine.PrimitiveComponent|SetbGenerateOverlapEvents (Variables|Default|GetSphere1) true))

(event EventTick
  (params (DeltaSeconds :type Float%20%28single-precision%29)))

(fn ConstructionScript)