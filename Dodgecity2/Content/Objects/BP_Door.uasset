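; BP_Door is a door actor that clears itself away once three referenced dummies have been defeated.
; When anything begins overlapping its Box component, nested checks test whether Dummy1, Dummy2 and Dummy3 all have Health at or below zero.
; If all three do, the door destroys itself; the check runs only on overlap and does not filter the overlapping actor.
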(event OnComponentBeginOverlap(Box)
  (params (OverlappedComponent :type Primitive%20Component%20Object%20Reference) (OtherActor :type Actor%20Object%20Reference) (OtherComp :type Primitive%20Component%20Object%20Reference) (OtherBodyIndex :type Integer) (bFromSweep :type Boolean) (SweepResult :type Hit%20Result%20Structure%20%28by%20ref%29))
  (if (<= (Variables|/Game/Objects/BP_Training_Dummy.BP_Training_Dummy_C|GetHealth (Variables|Default|GetDummy1)) 0.0)
    (if (<= (Variables|/Game/Objects/BP_Training_Dummy.BP_Training_Dummy_C|GetHealth (Variables|Default|GetDummy2)) 0.0)
      (if (<= (Variables|/Game/Objects/BP_Training_Dummy.BP_Training_Dummy_C|GetHealth (Variables|Default|GetDummy3)) 0.0)
        (Actor|DestroyActor)))))

(fn ConstructionScript)