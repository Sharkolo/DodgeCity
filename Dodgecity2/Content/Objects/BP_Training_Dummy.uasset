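; BP_Training_Dummy is a character target that loses health when a BP_Dodge_Ball overlaps it.
; Each such overlap subtracts a fixed amount from Health, which Tick polls for reaching zero.
; A one-shot flag then triggers mesh ragdoll physics and disables movement.
; After a short delay, it toggles visibility on the capsule and its children and turns off capsule collision, leaving the actor undestroyed.
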(event EventBeginPlay)

(event EventTick
  (params (DeltaSeconds :type Float%20%28single-precision%29))
  (bind _capsulecomponent (Variables|Collision|GetCapsuleComponent))
  (if (<= (Variables|Default|GetHealth) 0.0)
    (if (Variables|Default|GetOnly%20once)
      (Variables|Default|SetOnly%20once false)
      (Physics|SetSimulatePhysics (Variables|Character|GetMesh) true)
      (Pawn|Components|CharacterMovement|DisableMovement (Variables|Character|GetCharacterMovement))
      (Utilities|FlowControl|Delay 2.0)
      (Rendering|ToggleVisibility _capsulecomponent true)
      (Collision|SetCollisionEnabled _capsulecomponent "NoCollision"))))

(event Collision|EventActorBeginOverlap
  (params (OtherActor :type Actor%20Object%20Reference))
  (if (== (Utilities|GetClass OtherActor) "/Game/Objects/BP_Dodge_Ball.BP_Dodge_Ball_C")
    (Variables|Default|SetHealth (- (Variables|Default|GetHealth) 25.0))))

(fn ConstructionScript)